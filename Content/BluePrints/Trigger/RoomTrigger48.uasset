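; RoomTrigger48 is a room trigger that lets AI enemies close and lock the room's door once the required pair count is inside.
; When a C_Enemy enters, it waits briefly, then toggles TargetDoor shut if the overlapping Character count matches the GameInstance PairCount and the door is open.
; At higher difficulties it waits again, rechecks the count, room, door, lock and timer state in the GameInstance, then calls LockEvent.
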(event `self.ReceiveActorBeginOverlap`
  (params (OtherActor :type "Actor Object Reference"))
  (bind _targetdoor (`self.TargetDoor`))
  (bind _targetdoor_2 (`self.TargetDoor`))
  (bind _asgi_my_game_instance (cast `/Game/GI_MyGameInstance` (`GameplayStatics.GetGameInstance`) :!pure true))
  (bind _asgi_my_game_instance_2 (cast `/Game/GI_MyGameInstance` (`GameplayStatics.GetGameInstance`) :!pure true))
  (cast `/Game/Characters/C_Enemy` OtherActor) ; AI 적군이 밟았을 때만 수행
  (`KismetSystemLibrary.Delay` 0.5)
  ;[1 1 1] AI - 짝짓기 인원수 충족시
  (if (== (`KismetArrayLibrary.Array_Length` (`self.GetOverlappingActors` "/Script/Engine.Character")) (`/Game/GI_MyGameInstance.PairCount` _asgi_my_game_instance))
    ;[1 1 1] AI - 문 닫기
    (if (`BlueprintMapLibrary.Map_Find` (`/Game/GI_MyGameInstance.bDoorOpened` _asgi_my_game_instance) (`self.RoomIndex`))
      (`/Engine/EditorBlueprintResources/StandardMacros.IsValid` _targetdoor_2
        (:`Is Valid`
          (`/Game/BluePrints/Door/door_048_Blueprint.DoorEvent` _targetdoor_2)
          ;[1 1 1] 어려움 난이도 이상만 인공지능의 잠금 수행
          (if (>= (`/Game/GI_MyGameInstance.Game_Difficulty` (cast `/Game/GI_MyGameInstance` (`GameplayStatics.GetGameInstance`) :!pure true)) 2)
            (`|ExecutionSequence`
              (:`then_0`
                (`KismetSystemLibrary.Delay` 1.0)
                ;[1 1 1] AI - 짝짓기 인원수 충족시
                (if (== (`KismetArrayLibrary.Array_Length` (`self.GetOverlappingActors` "/Script/Engine.Character")) (`/Game/GI_MyGameInstance.PairCount` (cast `/Game/GI_MyGameInstance` (`GameplayStatics.GetGameInstance`) :!pure true)))
                  ;[1 1 1] AI - 문 잠금
                  (if (`/Game/GI_MyGameInstance.All_LockDoor` _asgi_my_game_instance_2)
                    _
                    (elif (`BlueprintMapLibrary.Map_Find` (`/Game/GI_MyGameInstance.IsRoomUse` _asgi_my_game_instance_2) (`self.RoomIndex`))
                      _
                      (elif (`BlueprintMapLibrary.Map_Find` (`/Game/GI_MyGameInstance.bLockDoor` _asgi_my_game_instance_2) (`self.RoomIndex`))
                        _
                        (elif (`BlueprintMapLibrary.Map_Find` (`/Game/GI_MyGameInstance.bDoorOpened` _asgi_my_game_instance_2) (`self.RoomIndex`))
                          _
                          (elif (not (<= (`/Game/GI_MyGameInstance.GI_RemainingTime` _asgi_my_game_instance_2) 0.5))
                            (`/Engine/EditorBlueprintResources/StandardMacros.IsValid` _targetdoor
                              (:`Is Valid`
                                (`/Game/BluePrints/Door/door_048_Blueprint.LockEvent` _targetdoor false)))))))))))))))))

(fn `UserConstructionScript`)