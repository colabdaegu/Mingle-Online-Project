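; RoomTrigger3 is a room trigger that shuts and locks its target door when AI enemies complete a required group size.
; On an enemy overlap, it compares the overlapping Character count with the game instance's NumberOfPerson.
; After a short delay, it checks the room's BDoorOpened entry and fires the door's DoorEvent.
; After another delay, it calls LockEvent only if the global lock, room-use and door-lock flags are all false.
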(event `self.ReceiveActorBeginOverlap`
  (params (OtherActor :type "Actor Object Reference"))
  (bind _targetdoor (`self.TargetDoor`))
  (bind _targetdoor_2 (`self.TargetDoor`))
  (bind _asgi_my_game_instance (cast `/Game/GI_MyGameInstance` (`GameplayStatics.GetGameInstance`) :!pure true))
  (bind _asgi_my_game_instance_2 (cast `/Game/GI_MyGameInstance` (`GameplayStatics.GetGameInstance`) :!pure true))
  (cast `/Game/Characters/C_Enemy` OtherActor) ; AI 적군이 밟았을 때만 수행
  ;[1 1 1] AI - 짝짓기 인원수 충족시
  (if (== (`KismetArrayLibrary.Array_Length` (`self.GetOverlappingActors` "/Script/Engine.Character")) (`/Game/GI_MyGameInstance.NumberOfPerson` _asgi_my_game_instance_2))
    ;[1 1 1] AI - 문 닫기
    (`KismetSystemLibrary.Delay` 0.5)
    (if (not (`BlueprintMapLibrary.Map_Find` (`/Game/GI_MyGameInstance.bDoorOpened` _asgi_my_game_instance_2) (`self.RoomIndex`)))
      (`/Engine/EditorBlueprintResources/StandardMacros.IsValid` _targetdoor_2
        (:`Is Valid`
          (`/Game/BluePrints/Door/door_003_Blueprint.DoorEvent` _targetdoor_2)
          ;[1 1 1] AI - 문 잠금
          (`KismetSystemLibrary.Delay` 0.5)
          (if (`/Game/GI_MyGameInstance.All_LockDoor` _asgi_my_game_instance)
            _
            (elif (`BlueprintMapLibrary.Map_Find` (`/Game/GI_MyGameInstance.IsRoomUse` _asgi_my_game_instance) (`self.RoomIndex`))
              _
              (elif (not (`BlueprintMapLibrary.Map_Find` (`/Game/GI_MyGameInstance.bLockDoor` _asgi_my_game_instance) (`self.RoomIndex`)))
                (`/Engine/EditorBlueprintResources/StandardMacros.IsValid` _targetdoor
                  (:`Is Valid`
                    (`/Game/BluePrints/Door/door_003_Blueprint.LockEvent` _targetdoor false)))))))))))

(fn `UserConstructionScript`)