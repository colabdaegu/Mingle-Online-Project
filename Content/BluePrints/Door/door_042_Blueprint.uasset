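; Interactive door 042 that BP_Contestant opens with Space and locks or unlocks with Q from the behind trigger while closed.
; Open and lock states live in GI_MyGameInstance maps keyed by DoorIndex, alongside room-use and global-lock checks.
; Overlap triggers gate input and prompts, while blocked attempts play a sound and flash a lock widget.
; Enemies in the front trigger start a timer for delayed opening of unlocked doors on higher difficulties.
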(event `DoorEvent`
  (bind _staticmeshcomponent (`self.StaticMeshComponent`))
  (bind _asgi_my_game_instance (cast `/Game/GI_MyGameInstance` (`GameplayStatics.GetGameInstance`) :!pure true))
  (if (`BlueprintMapLibrary.Map_Find` (`/Game/GI_MyGameInstance.bDoorOpened` _asgi_my_game_instance) (`self.DoorIndex`))
    (`self.K2_SetActorRotation` (struct))
    (`GameplayStatics.SpawnSoundAttached` "/Game/SoundFiles/Close-the-Door.Close-the-Door" _staticmeshcomponent "None" (0.0 0.0 0.0) (struct) "KeepRelativeOffset" false 1.0 1.0 0.0 "/Game/SoundFiles/Attenuations/SA_Far_Interaction.SA_Far_Interaction" null)
    (`BlueprintMapLibrary.Map_Add` (`/Game/GI_MyGameInstance.bDoorOpened` _asgi_my_game_instance) (`self.DoorIndex`))
    (else
      (`self.K2_SetActorRotation` (struct :`Yaw` -90.0))
      (`GameplayStatics.SpawnSoundAttached` "/Game/SoundFiles/Open-the-Door.Open-the-Door" _staticmeshcomponent "None" (0.0 0.0 0.0) (struct) "KeepRelativeOffset" false 1.0 1.0 0.0 "/Game/SoundFiles/Attenuations/SA_Far_Interaction.SA_Far_Interaction" null)
      (`BlueprintMapLibrary.Map_Add` (`/Game/GI_MyGameInstance.bDoorOpened` _asgi_my_game_instance) (`self.DoorIndex`) true))))

(event `LockEvent`
  (params (showWidget :type Boolean))
  (bind _asgi_my_game_instance (cast `/Game/GI_MyGameInstance` (`GameplayStatics.GetGameInstance`) :!pure true))
  (if (`BlueprintMapLibrary.Map_Find` (`/Game/GI_MyGameInstance.bLockDoor` _asgi_my_game_instance) (`self.DoorIndex`))
    (`GameplayStatics.SpawnSoundAttached` "/Game/SoundFiles/Unlock-the-Door.Unlock-the-Door" (`self.StaticMeshComponent`) "None" (0.0 0.0 0.0) (struct) "KeepRelativeOffset" false 1.0 1.0 0.0 "/Game/SoundFiles/Attenuations/SA_Near_Interaction.SA_Near_Interaction" null)
    (`BlueprintMapLibrary.Map_Add` (`/Game/GI_MyGameInstance.bLockDoor` _asgi_my_game_instance) (`self.DoorIndex`))
    (else
      (if showWidget
        (`self.Lock Widget`)
        (else
          (`GameplayStatics.SpawnSoundAttached` "/Game/SoundFiles/Lock-the-Door.Lock-the-Door" (`self.StaticMeshComponent`) "None" (0.0 0.0 0.0) (struct) "KeepRelativeOffset" false 1.0 1.0 0.0 "/Game/SoundFiles/Attenuations/SA_Near_Interaction.SA_Near_Interaction" null)))
      (`BlueprintMapLibrary.Map_Add` (`/Game/GI_MyGameInstance.bLockDoor` _asgi_my_game_instance) (`self.DoorIndex`) true))))

(event `self.door_042_Trigger.OnComponentBeginOverlap`
  (params (OverlappedComponent :type "PrimitiveComponent Object Reference") (OtherActor :type "Actor Object Reference") (OtherComp :type "PrimitiveComponent Object Reference") (OtherBodyIndex :type Integer) (bFromSweep :type Boolean) (SweepResult :type "HitResult Structure (by ref)"))
  (cast `/Game/ThirdPerson/Blueprints/BP_Contestant` OtherActor)
  (`/Engine/EditorBlueprintResources/StandardMacros.IsValid` (`self.DoorWidget`)
    (:`Is Not Valid`
      (bind _returnvalue (`|CreateWidget` "/Game/Widgets/WBP_Door.WBP_Door_C"))
      (bind _output_get (set `self.DoorWidget` _returnvalue))
      (`UserWidget.AddToViewport` _output_get 0)
      (set `self.bPlayerInTrigger` true)
      (`self.EnableInput` (`GameplayStatics.GetPlayerController` 0)))))

(event `self.door_042_Trigger.OnComponentEndOverlap`
  (params (OverlappedComponent :type "PrimitiveComponent Object Reference") (OtherActor :type "Actor Object Reference") (OtherComp :type "PrimitiveComponent Object Reference") (OtherBodyIndex :type Integer))
  (bind _doorwidget (`self.DoorWidget`))
  (cast `/Game/ThirdPerson/Blueprints/BP_Contestant` OtherActor)
  (`/Engine/EditorBlueprintResources/StandardMacros.IsValid` _doorwidget
    (:`Is Valid`
      (`Widget.RemoveFromParent` _doorwidget)
      (set `self.DoorWidget` null)
      (set `self.bPlayerInTrigger` false)
      (`self.DisableInput` (`GameplayStatics.GetPlayerController` 0)))))

(event `self.behind_042_Trigger.OnComponentBeginOverlap`
  (params (OverlappedComponent :type "PrimitiveComponent Object Reference") (OtherActor :type "Actor Object Reference") (OtherComp :type "PrimitiveComponent Object Reference") (OtherBodyIndex :type Integer) (bFromSweep :type Boolean) (SweepResult :type "HitResult Structure (by ref)"))
  (cast `/Game/ThirdPerson/Blueprints/BP_Contestant` OtherActor)
  (set `self.bPlayerInLockTrigger` true))

(event `self.behind_042_Trigger.OnComponentEndOverlap`
  (params (OverlappedComponent :type "PrimitiveComponent Object Reference") (OtherActor :type "Actor Object Reference") (OtherComp :type "PrimitiveComponent Object Reference") (OtherBodyIndex :type Integer))
  (cast `/Game/ThirdPerson/Blueprints/BP_Contestant` OtherActor)
  (set `self.bPlayerInLockTrigger` false))

(event `Key|SpaceBar`
  (params (Key :type "Key Structure"))
  (bind _asgi_my_game_instance (cast `/Game/GI_MyGameInstance` (`GameplayStatics.GetGameInstance`) :!pure true))
  (:`Pressed`
    (if (`self.bPlayerInTrigger`)
      (if (`/Game/GI_MyGameInstance.All_LockDoor` _asgi_my_game_instance)
        (`self.All Lock Widget`)
        (elif (`BlueprintMapLibrary.Map_Find` (`/Game/GI_MyGameInstance.IsRoomUse` _asgi_my_game_instance) (`self.DoorIndex`))
          (`self.Lock Widget` :!label _label)
          (elif (`BlueprintMapLibrary.Map_Find` (`/Game/GI_MyGameInstance.bLockDoor` _asgi_my_game_instance) (`self.DoorIndex`))
            (goto _label)
            (else
              (`self.DoorEvent`) ; 개별 문 열기/닫기
            )))))))

(event `Key|Q`
  (params (Key :type "Key Structure"))
  (bind _asgi_my_game_instance (cast `/Game/GI_MyGameInstance` (`GameplayStatics.GetGameInstance`) :!pure true))
  (:`Pressed`
    (if (`self.bPlayerInLockTrigger`)
      (if (`BlueprintMapLibrary.Map_Find` (`/Game/GI_MyGameInstance.bDoorOpened` _asgi_my_game_instance) (`self.DoorIndex`))
        _
        (elif (`/Game/GI_MyGameInstance.All_LockDoor` _asgi_my_game_instance)
          _
          (elif (not (`BlueprintMapLibrary.Map_Find` (`/Game/GI_MyGameInstance.IsRoomUse` _asgi_my_game_instance) (`self.DoorIndex`)))
            (`self.LockEvent` true) ; 개별 문 잠금/해제
          ))))))

(event `Lock Widget`
  (bind _alllockwidget (`self.AllLockWidget`))
  (bind _lockwidget (`self.LockWidget`))
  (`GameplayStatics.SpawnSoundAttached` "/Game/SoundFiles/Lock-the-Door.Lock-the-Door" (`self.StaticMeshComponent`) "None" (0.0 0.0 0.0) (struct) "KeepRelativeOffset" false 1.0 1.0 0.0 "/Game/SoundFiles/Attenuations/SA_Near_Interaction.SA_Near_Interaction" null)
  (`/Engine/EditorBlueprintResources/StandardMacros.IsValid` (`self.LockWidget`)
    (:`Is Not Valid`
      (`/Engine/EditorBlueprintResources/StandardMacros.IsValid` _alllockwidget
        (:`Is Valid`
          (`Widget.RemoveFromParent` _alllockwidget)
          (set `self.AllLockWidget` null))
        (:`Is Not Valid`
          _))
      (bind _returnvalue (`|CreateWidget` "/Game/Widgets/WBP_Lock.WBP_Lock_C"))
      (bind _output_get (set `self.LockWidget` _returnvalue))
      (`UserWidget.AddToViewport` _output_get 0)
      (`KismetSystemLibrary.Delay` 1.0)
      (`/Engine/EditorBlueprintResources/StandardMacros.IsValid` _lockwidget
        (:`Is Valid`
          (`Widget.RemoveFromParent` _lockwidget)
          (set `self.LockWidget` null))))))

(event `All Lock Widget`
  (bind _alllockwidget (`self.AllLockWidget`))
  (bind _lockwidget (`self.LockWidget`))
  (`GameplayStatics.SpawnSoundAttached` "/Game/SoundFiles/Lock-the-Door.Lock-the-Door" (`self.StaticMeshComponent`) "None" (0.0 0.0 0.0) (struct) "KeepRelativeOffset" false 1.0 1.0 0.0 "/Game/SoundFiles/Attenuations/SA_Near_Interaction.SA_Near_Interaction" null)
  (`/Engine/EditorBlueprintResources/StandardMacros.IsValid` (`self.AllLockWidget`)
    (:`Is Not Valid`
      (`/Engine/EditorBlueprintResources/StandardMacros.IsValid` _lockwidget
        (:`Is Valid`
          (`Widget.RemoveFromParent` _lockwidget)
          (set `self.LockWidget` null))
        (:`Is Not Valid`
          _))
      (bind _returnvalue (`|CreateWidget` "/Game/Widgets/WBP_AllLock.WBP_AllLock_C"))
      (bind _output_get (set `self.AllLockWidget` _returnvalue))
      (`UserWidget.AddToViewport` _output_get 0)
      (`KismetSystemLibrary.Delay` 1.0)
      (`/Engine/EditorBlueprintResources/StandardMacros.IsValid` _alllockwidget
        (:`Is Valid`
          (`Widget.RemoveFromParent` _alllockwidget)
          (set `self.AllLockWidget` null))))))

(event `self.front_042_Trigger.OnComponentBeginOverlap`
  (params (OverlappedComponent :type "PrimitiveComponent Object Reference") (OtherActor :type "Actor Object Reference") (OtherComp :type "PrimitiveComponent Object Reference") (OtherBodyIndex :type Integer) (bFromSweep :type Boolean) (SweepResult :type "HitResult Structure (by ref)"))
  (cast `/Game/Characters/C_Enemy` OtherActor) ; AI 적군이 밟았을 때만 수행
  (set `self.AiInFrontTrigger` true)
  (`KismetSystemLibrary.K2_ClearAndInvalidateTimerHandle` (`self.HoldHandle`))
  (bind _returnvalue (`KismetSystemLibrary.K2_SetTimerDelegate` (`|CreateDelegate` :!event `AI Door Delay Open Event`) 2.0))
  (set `self.HoldHandle` _returnvalue))

(event `self.front_042_Trigger.OnComponentEndOverlap`
  (params (OverlappedComponent :type "PrimitiveComponent Object Reference") (OtherActor :type "Actor Object Reference") (OtherComp :type "PrimitiveComponent Object Reference") (OtherBodyIndex :type Integer))
  (cast `/Game/Characters/C_Enemy` OtherActor) ; AI 적군이 밟았을 때만 수행
  (set `self.AiInFrontTrigger` false)
  (`KismetSystemLibrary.K2_ClearAndInvalidateTimerHandle` (`self.HoldHandle`)))

(event `AI Door Delay Open Event`
  (bind _asgi_my_game_instance (cast `/Game/GI_MyGameInstance` (`GameplayStatics.GetGameInstance`) :!pure true))
  (if (and (`self.AiInFrontTrigger`) (>= (`/Game/GI_MyGameInstance.Game_Difficulty` (cast `/Game/GI_MyGameInstance` (`GameplayStatics.GetGameInstance`) :!pure true)) 2))
    (if (`/Game/GI_MyGameInstance.All_LockDoor` _asgi_my_game_instance)
      _
      (elif (`BlueprintMapLibrary.Map_Find` (`/Game/GI_MyGameInstance.IsRoomUse` _asgi_my_game_instance) (`self.DoorIndex`))
        _
        (elif (`BlueprintMapLibrary.Map_Find` (`/Game/GI_MyGameInstance.bLockDoor` _asgi_my_game_instance) (`self.DoorIndex`))
          _
          (elif (not (`BlueprintMapLibrary.Map_Find` (`/Game/GI_MyGameInstance.bDoorOpened` _asgi_my_game_instance) (`self.DoorIndex`)))
            (`self.DoorEvent`)))))))

(fn `UserConstructionScript`)